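; BP_DisableSphere is a one-way trigger sphere that switches off a linked target actor when the third-person character enters its ProximityTrigger.
; On overlap it hides its own Sphere, removes that mesh's collision, then hides TargetToDisable and disables its collision.
; If both target and ManagerReference are valid, SphereID selects one of three Dispositivo (device) flags to set on the manager, which then runs CheckDevices.
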(event `self.ProximityTrigger.OnComponentBeginOverlap`
  (params (OverlappedComponent :type "PrimitiveComponent Object Reference") (OtherActor :type "Actor Object Reference") (OtherComp :type "PrimitiveComponent Object Reference") (OtherBodyIndex :type Integer) (bFromSweep :type Boolean) (SweepResult :type "HitResult Structure (by ref)"))
  (bind _managerreference (`self.ManagerReference`))
  (cast `/Game/ThirdPerson/Blueprints/BP_ThirdPersonCharacter` OtherActor)
  (`SceneComponent.SetVisibility` (`self.Sphere`) false false)
  (`PrimitiveComponent.SetCollisionEnabled` (`self.Sphere`) "NoCollision")
  (`/Engine/EditorBlueprintResources/StandardMacros.IsValid` (`self.TargetToDisable`)
    (:`Is Valid`
      (`self.SetActorHiddenInGame` (`self.TargetToDisable`) true)
      (`self.SetActorEnableCollision` (`self.TargetToDisable`) false)
      (`/Engine/EditorBlueprintResources/StandardMacros.IsValid` (`self.ManagerReference`)
        (:`Is Valid`
          (switch `int` (`self.SphereID`)
            (:`1`
              (bind _output_get (set `self.ManagerReference` _managerreference))
              (set `/Game/Fungal_Forest/Blueprints/BP_CampoDeFuerza.Dispositivo_1` true _output_get))
            (:`2`
              (bind _output_get_2 (set `self.ManagerReference` _managerreference))
              (set `/Game/Fungal_Forest/Blueprints/BP_CampoDeFuerza.Dispositivo_2` true _output_get_2))
            (:`3`
              (bind _output_get_3 (set `self.ManagerReference` _managerreference))
              (set `/Game/Fungal_Forest/Blueprints/BP_CampoDeFuerza.Dispositivo_3` true _output_get_3)))
          (`/Game/Fungal_Forest/Blueprints/BP_CampoDeFuerza.CheckDevices` (`self.ManagerReference`)))))))

(fn `UserConstructionScript`)