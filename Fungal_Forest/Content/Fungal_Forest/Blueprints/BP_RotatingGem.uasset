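; BP_RotatingGem is a gem pickup that spins in place and disappears when the player character touches it.
; Tick yaws GemMesh locally by RotationSpeed scaled with delta time, keeping the spin frame-rate independent.
; Overlapping PickupTrigger with a BP_ThirdPersonCharacter hides the mesh, disables trigger collision and destroys the actor, without awarding or notifying anything.
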(event `self.ReceiveTick`
  (params (DeltaSeconds :type "Float (single-precision)"))
  (`SceneComponent.K2_AddLocalRotation` (`self.GemMesh`) (`KismetMathLibrary.MakeRotator` 0.0 0.0 (* DeltaSeconds (`self.Rotation Speed`))) false false))

(event `self.PickupTrigger.OnComponentBeginOverlap`
  (params (OverlappedComponent :type "PrimitiveComponent Object Reference") (OtherActor :type "Actor Object Reference") (OtherComp :type "PrimitiveComponent Object Reference") (OtherBodyIndex :type Integer) (bFromSweep :type Boolean) (SweepResult :type "HitResult Structure (by ref)"))
  (cast `/Game/ThirdPerson/Blueprints/BP_ThirdPersonCharacter` OtherActor)
  (`SceneComponent.SetVisibility` (`self.GemMesh`) false false)
  (`PrimitiveComponent.SetCollisionEnabled` (`self.PickupTrigger`) "NoCollision")
  (`self.K2_DestroyActor`))

(fn `UserConstructionScript`)