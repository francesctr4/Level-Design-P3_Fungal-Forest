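; BP_CrystalVariant is a crystal that, when the third-person character comes near, switches to its active material and removes a linked actor.
; BeginPlay applies the default material and, if ActorToEnable is valid, shows it with collision and sizes the proximity sphere.
; On overlap, that actor is hidden and loses collision, despite its name.
; Nothing here reverts this: ResetTimerHandle is cleared but never set.
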(event `self.ReceiveBeginPlay`
  (bind _actortoenable (`self.ActorToEnable`))
  (`PrimitiveComponent.SetMaterial` (`self.CrystalMesh`) 0 (`self.DefaultMaterial`))
  (`/Engine/EditorBlueprintResources/StandardMacros.IsValid` _actortoenable
    (:`Is Valid`
      (`self.SetActorHiddenInGame` _actortoenable false)
      (`self.SetActorEnableCollision` _actortoenable true)
      (`SphereComponent.SetSphereRadius` (`self.ProximitySphere`) (`self.SphereRadius`) true))))

(event `self.ProximitySphere.OnComponentBeginOverlap`
  (params (OverlappedComponent :type "PrimitiveComponent Object Reference") (OtherActor :type "Actor Object Reference") (OtherComp :type "PrimitiveComponent Object Reference") (OtherBodyIndex :type Integer) (bFromSweep :type Boolean) (SweepResult :type "HitResult Structure (by ref)"))
  (bind _actortoenable (`self.ActorToEnable`))
  (cast `/Game/ThirdPerson/Blueprints/BP_ThirdPersonCharacter` OtherActor)
  (`PrimitiveComponent.SetMaterial` (`self.CrystalMesh`) 0 (`self.ActiveMaterial`))
  (`KismetSystemLibrary.K2_ClearAndInvalidateTimerHandle` (`self.ResetTimerHandle`))
  (`/Engine/EditorBlueprintResources/StandardMacros.IsValid` _actortoenable
    (:`Is Valid`
      (`self.SetActorHiddenInGame` _actortoenable true)
      (`self.SetActorEnableCollision` _actortoenable false))))

(fn `UserConstructionScript`)