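; Force field controller for the Fungal Forest that opens a barrier once three devices are all set.
; A CheckDevices event tests the three Dispositivo flags, then hides the referenced CampoDeFuerza actor and disables its collision if all are true, or restores both otherwise.
; The file neither sets the flags nor calls the event, and BeginPlay, Tick and the construction script are empty.
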(event `CheckDevices`
  (if (and (`self.Dispositivo_1`) (`self.Dispositivo_2`) (`self.Dispositivo_3`))
    (`self.SetActorHiddenInGame` (`self.Campo de Fuerza`) true)
    (`self.SetActorEnableCollision` (`self.Campo de Fuerza`) false)
    (else
      (`self.SetActorHiddenInGame` (`self.Campo de Fuerza`) false)
      (`self.SetActorEnableCollision` (`self.Campo de Fuerza`) true))))

(fn `UserConstructionScript`)